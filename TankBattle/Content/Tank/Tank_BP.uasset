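; Player-controllable tank Blueprint that maps input to aiming, movement and firing components.
; BeginPlay initializes TankAiming with the turret and barrel, and TankMovement with the left and right tracks.
; Aim axes rotate the azimuth gimbal in yaw and the spring arm in pitch, while move axes pass forward and clockwise intents to TankMovement.
; The Fire press calls TankAiming.Fire.
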(event EventBeginPlay
  (Class|TankAimingComponent|Initialize (Variables|Default|GetTankAiming) (Variables|Default|GetTurret) (Variables|Default|GetBarrel))
  (Class|TankMovementComponent|Initialize (Variables|Default|GetTankMovement) (Variables|Default|GetLeftTrack) (Variables|Default|GetRightTrack)))

(event Input|ActionEvents|InputActionFire
  (params (Key :type Key%20Structure))
  ;[1 1 1] Aiming Input binding
  (:Pressed
    (Class|TankAimingComponent|Fire (Variables|Default|GetTankAiming))))

(event Input|AxisEvents|InputAxisAimAzimuth
  (params (AxisValue :type Float%20%28single-precision%29))
  ;[1 1 1] Aiming Input binding
  (Transformation|AddLocalRotation (Variables|Default|GetAzimuthGimbal) (Math|Rotator|MakeRotator 0.0 0.0 AxisValue) false false))

(event Input|AxisEvents|InputAxisMoveClockwise
  (params (AxisValue :type Float%20%28single-precision%29))
  ;[1 1 1] Movement input binding
  (Class|TankMovementComponent|IntendTurnClockwise (Variables|Default|GetTankMovement) AxisValue))

(event Input|AxisEvents|InputAxisAimElevation
  (params (AxisValue :type Float%20%28single-precision%29))
  ;[1 1 1] Aiming Input binding
  (Transformation|AddLocalRotation (Variables|Default|GetSpringArm) (Math|Rotator|MakeRotator 0.0 AxisValue 0.0) false false))

(event Input|AxisEvents|InputAxisMoveForward
  (params (AxisValue :type Float%20%28single-precision%29))
  ;[1 1 1] Movement input binding
  (Class|TankMovementComponent|IntendMoveForward (Variables|Default|GetTankMovement) AxisValue))

(fn ConstructionScript)